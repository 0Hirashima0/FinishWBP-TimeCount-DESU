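; BP_IceChara is an ice character Blueprint that runs a game countdown and handles pausing.
; Tick uses a one-second Delay as a timer, decrementing and printing Seconds, then swaps all widgets for a finish screen and pauses the game once it drops below zero.
; The Pause input replaces all widgets with WBP_Pause, shows the cursor, switches to UI-only input and pauses the game.
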(event `self.ReceiveTick`
  (params (DeltaSeconds :type "Float (single-precision)"))
  (`KismetSystemLibrary.Delay` 1.0)
  (bind _output_get (set `self.Seconds` (- (`self.Seconds`) 1)))
  (`KismetSystemLibrary.PrintString` (`KismetStringLibrary.Conv_IntToString` _output_get))
  (if (< (`self.Seconds`) 0)
    (`WidgetLayoutLibrary.RemoveAllWidgets`)
    (bind _returnvalue (`|CreateWidget` "/Game/IceCatch/UIまとめ/WBP_Finish.WBP_Finish_C"))
    (`UserWidget.AddToViewport` _returnvalue 0)
    (set `PlayerController.bShowMouseCursor` false (`GameplayStatics.GetPlayerController` 0))
    (`GameplayStatics.SetGamePaused` true)))

(event `InputAction|Pause`
  (params (Key :type "Key Structure"))
  (bind _returnvalue (`GameplayStatics.GetPlayerController` 0))
  (:`Pressed`
    (`WidgetLayoutLibrary.RemoveAllWidgets`)
    (bind _returnvalue_2 (`|CreateWidget` "/Game/IceCatch/UIまとめ/WBP_Pause.WBP_Pause_C"))
    (`UserWidget.AddToViewport` _returnvalue_2 0)
    (set `PlayerController.bShowMouseCursor` true _returnvalue)
    (`WidgetBlueprintLibrary.SetInputMode_UIOnlyEx` _returnvalue null) ; UI用のモードに切り替える
    ;[0.3886 1 0.7649] できた！！多分！！！
    (`GameplayStatics.SetGamePaused` true)))

(fn `UserConstructionScript`)